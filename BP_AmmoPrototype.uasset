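; Prototype projectile actor that deals damage on contact and explodes with a fireworks burst and sound.
; On spawn it records its start time, sets its attack value and self-destructs after a short delay.
; Box overlaps are ignored briefly after spawn; later ones damage damageable actors, then trigger the same self-destruct effect and destroy.
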(event `self.ReceiveBeginPlay`
  ;[1 0 0.1406] Self Destruct
  (set `self.lifetime` (`KismetSystemLibrary.GetGameTimeInSeconds`))
  (set `self.AttackPoint` 10)
  (`KismetSystemLibrary.Delay` 2.0)
  (`self.SelfDestruct`))

(event `SelfDestruct`
  ;[0.5234 0 1] SelfDestruct
  (`GameplayStatics.SpawnEmitterAtLocation` "/Game/TS_Fireworks/Particles/PS_TS_Fireworks_Burst_Chrys.PS_TS_Fireworks_Burst_Chrys" (`self.K2_GetActorLocation`) (struct) (0.5 0.5 0.5))
  (`GameplayStatics.PlaySound2D` "/Game/StarterContent/Audio/Explosion_Cue.Explosion_Cue" 1.0 1.0 0.0 null null)
  (`self.K2_DestroyActor`))

(event `self.Box.OnComponentBeginOverlap`
  (params (OverlappedComponent :type "PrimitiveComponent Object Reference") (OtherActor :type "Actor Object Reference") (OtherComp :type "PrimitiveComponent Object Reference") (OtherBodyIndex :type Integer) (bFromSweep :type Boolean) (SweepResult :type "HitResult Structure (by ref)"))
  ;[0.8516 1 0] Comment
  (if (> (- (`KismetSystemLibrary.GetGameTimeInSeconds`) (`self.lifetime`)) 0.1)
    (if (`Actor.bCanBeDamaged` OtherActor)
      (`GameplayStatics.ApplyDamage` OtherActor (`KismetMathLibrary.Conv_IntToDouble` (`self.AttackPoint`)))
      (`self.SelfDestruct`)
      (else
        (`self.SelfDestruct`)))))

(fn `UserConstructionScript`)