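; BP_RedBloodCell is a red blood cell actor that drifts in a straight line and reverses when it touches something.
; BeginPlay builds a random 3D direction scaled by Speed, without normalizing it, so the pace varies per cell.
; Tick applies that offset with sweep every frame, unscaled by delta time, so movement depends on frame rate.
; The Box component's begin-overlap event negates the direction.
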(event `self.ReceiveBeginPlay`
  (set `self.Direction` (* (`KismetMathLibrary.MakeVector` (`KismetMathLibrary.RandomFloatInRange` -1.0 1.0) (`KismetMathLibrary.RandomFloatInRange` -1.0 1.0) (`KismetMathLibrary.RandomFloatInRange` -1.0 1.0)) (`self.Speed`))))

(event `self.ReceiveTick`
  (params (DeltaSeconds :type "Float (single-precision)"))
  (`self.K2_AddActorWorldOffset` (`self.Direction`) true))

(event `self.Box.OnComponentBeginOverlap`
  (params (OverlappedComponent :type "PrimitiveComponent Object Reference") (OtherActor :type "Actor Object Reference") (OtherComp :type "PrimitiveComponent Object Reference") (OtherBodyIndex :type Integer) (bFromSweep :type Boolean) (SweepResult :type "HitResult Structure (by ref)"))
  (set `self.Direction` (* (`self.Direction`) -1)))

(fn `UserConstructionScript`)