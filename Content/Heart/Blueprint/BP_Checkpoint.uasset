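; BP_Checkpoint is a one-time checkpoint that updates the player's respawn point when touched.
; When a DemoThirdPersonCharacter first overlaps the Box, it sets that character's SpawnLocation to a point above the Cylinder, keeping the Cylinder's rotation.
; It then latches HasHitBefore, prints a confirmation and plays a timeline that spins the Antenna by adding local yaw each update.
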(event `self.Box.OnComponentBeginOverlap`
  (params (OverlappedComponent :type "PrimitiveComponent Object Reference") (OtherActor :type "Actor Object Reference") (OtherComp :type "PrimitiveComponent Object Reference") (OtherBodyIndex :type Integer) (bFromSweep :type Boolean) (SweepResult :type "HitResult Structure (by ref)"))
  (if (not (`self.hasHitBefore`))
    (bind _asdemo_third_person_character (cast `/Game/ThirdPersonCPP/Blueprints/DemoThirdPersonCharacter` OtherActor))
    (set `/Game/ThirdPersonCPP/Blueprints/DemoThirdPersonCharacter.spawnLocation` (`KismetMathLibrary.MakeTransform` (+ (.location (`SceneComponent.K2_GetComponentToWorld` (`self.cylinder`))) (0.0 0.0 200.0)) (.rotation (`SceneComponent.K2_GetComponentToWorld` (`self.cylinder`)))) _asdemo_third_person_character)
    (set `self.hasHitBefore` true)
    (`KismetSystemLibrary.PrintString` "checkpoint reached")
    (bind (_direction _newtrack_0) (`Timeline|Timeline_0` :!via `PlayFromStart`)
      (:`Update`
        (`SceneComponent.K2_AddLocalRotation` (`self.antenna`) (`KismetMathLibrary.MakeRotator` 0.0 0.0 _newtrack_0) false false)))))

(fn `UserConstructionScript`)