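; Basic enemy Blueprint for BodyDefenseForce that attacks and dies from any damage event, with a health variable still to be added.
; OnTakeDamage calls OnDeath, which runs once via IsDead, disables mesh collision, stops the AI controller's brain logic, then destroys the actor after a short delay.
; DoAttack switches mesh collision to query-only while attacking, with a debug print, and disables it otherwise.
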(event `OnTakeDamage`
  (`self.OnDeath`))

(event `OnDeath`
  (if (not (`self.IsDead`))
    (`PrimitiveComponent.SetCollisionEnabled` (`self.Mesh`) "NoCollision")
    (set `self.IsDead` true)
    (`BrainComponent.StopLogic` (`AIController.BrainComponent` (`AIBlueprintHelperLibrary.GetAIController` self)) "")
    (`KismetSystemLibrary.Delay` 1.5)
    (`self.K2_DestroyActor`)))

(fn `DoAttack`
  (params (IsAttacking :type Boolean))
  (bind _mesh (`self.Mesh`))
  (if IsAttacking
    (`PrimitiveComponent.SetCollisionEnabled` _mesh "QueryOnly")
    (`KismetSystemLibrary.PrintString` "Attacking")
    (else
      (`PrimitiveComponent.SetCollisionEnabled` _mesh "NoCollision")
      (set `self.IsAttacking` false))))

(fn `UserConstructionScript`)