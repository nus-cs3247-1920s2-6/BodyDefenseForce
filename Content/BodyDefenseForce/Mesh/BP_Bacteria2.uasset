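; BP_Bacteria2 is a bacteria actor in BodyDefenseForce that deals contact damage and can be killed.
; Its Sphere applies DamagePower to any actor that begins overlapping it, with no filtering or repeat ticks.
; AnyDamage feeds absolute, truncated damage into DealDamage, which lowers Health and destroys the actor at zero or below.
; BeginPlay fills Health from MaxHealth and derives Name from a substring of the object's name.
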(event `self.Sphere.OnComponentBeginOverlap`
  (params (OverlappedComponent :type "PrimitiveComponent Object Reference") (OtherActor :type "Actor Object Reference") (OtherComp :type "PrimitiveComponent Object Reference") (OtherBodyIndex :type Integer) (bFromSweep :type Boolean) (SweepResult :type "HitResult Structure (by ref)"))
  ;[0 1 0.7891] Deal close combat damage to nearby actors
  (`GameplayStatics.ApplyDamage` OtherActor (`KismetMathLibrary.Conv_IntToDouble` (`self.DamagePower`))))

(event `self.ReceiveAnyDamage`
  (params (Damage :type "Float (single-precision)") (DamageType :type "DamageType Object Reference") (InstigatedBy :type "Controller Object Reference") (DamageCauser :type "Actor Object Reference"))
  ;[1 0 0.1172] Comment
  (`self.Deal Damage` (`KismetMathLibrary.FTrunc` (`KismetMathLibrary.Abs` Damage))))

(event `Actor Die`
  ;[1 0.8438 0] Comment
  (if (<= (`self.Health`) 0)
    (`self.K2_DestroyActor`)))

(event `Deal Damage`
  (params (Damage :type Integer))
  ;[0 1 0.2031] Comment
  (bind _output_get (set `self.Health` (- (`self.Health`) Damage)))
  (if (<= _output_get 0)
    (`self.K2_DestroyActor`)))

(event `self.ReceiveBeginPlay`
  ;[0.125 0 1] Comment
  (set `self.Name` (`KismetStringLibrary.GetSubstring` (`KismetStringLibrary.Conv_ObjectToString` self) 3 11))
  (set `self.Health` (`self.MaxHealth`)))

(fn `UserConstructionScript`)