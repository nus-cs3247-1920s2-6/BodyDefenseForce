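; BP_charge is an enemy character that wanders randomly, rams the player and can multiply over time.
; An overlap on its Sphere starts a per-tick force toward the player until AttackField overlaps, which knocks the player back and deals damage.
; When duplication is enabled, a Tick timer periodically spawns another BP_charge nearby.
; Health is randomized at spawn; death triggers ragdoll physics, delayed destruction and an XP award.
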(event `AISearch`
  ;[1 0 0.04687] Search
  (bind _asdemo_third_person_character (cast `/Game/ThirdPersonCPP/Blueprints/DemoThirdPersonCharacter` (`GameplayStatics.GetPlayerCharacter` 0)))
  (`|AIMoveTo` self (0.0 0.0 0.0) _asdemo_third_person_character :!label _label
    (:`OnFail`
      (`KismetSystemLibrary.Delay` 1.0)
      (goto _label))))

(event `self.ReceiveBeginPlay`
  (bind _returnvalue (`KismetMathLibrary.RandomIntegerInRange` 10 30))
  ;[0.875 0 1] Set Initialization
  (set `self.BornTime` (`KismetSystemLibrary.GetGameTimeInSeconds`))
  (set `self.MaxHealth` (- _returnvalue (mod _returnvalue 5)))
  (set `self.Health` (`self.MaxHealth`))
  (`KismetSystemLibrary.Delay` 0.3)
  (set `CharacterMovementComponent.MaxWalkSpeed` (`KismetMathLibrary.RandomFloatInRange` 400.0 600.0) (`self.CharacterMovement`))
  (`self.RandomWalk`))

(event `RandomWalk`
  (`|AIMoveTo` self (`NavigationSystemV1.K2_GetRandomReachablePointInRadius` (`self.K2_GetActorLocation`) 300.0 null null) null :!label _label_2
    (:`OnSuccess`
      (if true
        (goto _label_2)))))

(event `self.ReceiveAnyDamage`
  (params (Damage :type "Float (single-precision)") (DamageType :type "DamageType Object Reference") (InstigatedBy :type "Controller Object Reference") (DamageCauser :type "Actor Object Reference"))
  ;[0.1016 1 0] Damage
  (bind _dead_ (message `/Game/ThirdPersonCPP/Blueprints/BPI_DamageCalculate.Damageint` self (`KismetMathLibrary.FTrunc` Damage)))
  (if _dead_
    (`MovementComponent.StopMovementImmediately` (`self.CharacterMovement`))
    (`GameplayStatics.PlaySoundAtLocation` "/Game/BodyDefenseForce/Audio/SoundEffect/Enemy/SW_Enemy_Dead_Mid.SW_Enemy_Dead_Mid" (`self.K2_GetActorLocation`) (struct) 1.0 1.0 0.0 null null null)
    (`PrimitiveComponent.SetSimulatePhysics` (`self.Mesh`) true)
    (`PrimitiveComponent.SetEnableGravity` (`self.Mesh`) true)
    (`KismetSystemLibrary.Delay` 0.5)
    (`self.K2_DestroyActor`)
    (bind _asdemo_third_person_character (cast `/Game/ThirdPersonCPP/Blueprints/DemoThirdPersonCharacter` (`GameplayStatics.GetPlayerCharacter` 0)))
    (`/Game/ThirdPersonCPP/Blueprints/DemoThirdPersonCharacter.AddXP` _asdemo_third_person_character (* (`self.MaxHealth`) 2.0))))

(event `self.Sphere.OnComponentBeginOverlap`
  (params (OverlappedComponent :type "PrimitiveComponent Object Reference") (OtherActor :type "Actor Object Reference") (OtherComp :type "PrimitiveComponent Object Reference") (OtherBodyIndex :type Integer) (bFromSweep :type Boolean) (SweepResult :type "HitResult Structure (by ref)"))
  (set `self.Charge?` true)
  (`NavMovementComponent.StopMovementKeepPathing` (`self.CharacterMovement`)))

(event `self.Sphere.OnComponentEndOverlap`
  (params (OverlappedComponent :type "PrimitiveComponent Object Reference") (OtherActor :type "Actor Object Reference") (OtherComp :type "PrimitiveComponent Object Reference") (OtherBodyIndex :type Integer))
  (set `self.Charge?` false)
  (set `self.Hit?` false)
  (`self.RandomWalk`))

(event `self.AttackField.OnComponentBeginOverlap`
  (params (OverlappedComponent :type "PrimitiveComponent Object Reference") (OtherActor :type "Actor Object Reference") (OtherComp :type "PrimitiveComponent Object Reference") (OtherBodyIndex :type Integer) (bFromSweep :type Boolean) (SweepResult :type "HitResult Structure (by ref)"))
  (if (`self.Charge?`)
    (set `self.Hit?` true)
    (bind _asdemo_third_person_character (cast `/Game/ThirdPersonCPP/Blueprints/DemoThirdPersonCharacter` (`GameplayStatics.GetPlayerCharacter` 0)))
    (`CharacterMovementComponent.AddImpulse` (`Character.CharacterMovement` _asdemo_third_person_character) (* (`KismetMathLibrary.Normal` (- (`self.K2_GetActorLocation` self) (`self.K2_GetActorLocation` (`GameplayStatics.GetPlayerCharacter` 0)))) -300000.0) false)
    (`GameplayStatics.ApplyDamage` (`GameplayStatics.GetPlayerCharacter` 0) 5.0 null self)))

(event `self.ReceiveTick`
  (params (DeltaSeconds :type "Float (single-precision)"))
  (`|ExecutionSequence`
    (:`then_0`
      (if (`self.Charge?`)
        (`self.Charge`)))
    (:`then_1`
      (if (`self.CanDuplicate?`)
        (if (`self.Duplicated?`)
          (set `self.Duplicated?` false)
          (set `self.BornTime` (`KismetSystemLibrary.GetGameTimeInSeconds`))
          (else
            (bind _output_get (set `self.TimeCircle` (- (`KismetSystemLibrary.GetGameTimeInSeconds`) (`self.BornTime`))))
            (if (> _output_get (`self.DuplicationTime`))
              (`AIBlueprintHelperLibrary.SpawnAIFromClass` "BP_charge_C" "/Game/BodyDefenseForce/AIController/AI_BT.AI_BT" (`NavigationSystemV1.K2_GetRandomLocationInNavigableRadius` (`self.K2_GetActorLocation`) 250.0 null null))
              (set `self.Duplicated?` true))))))))

(fn `Charge`
  (if (not (`self.Hit?`))
    (`CharacterMovementComponent.AddForce` (`self.CharacterMovement`) (* (`KismetMathLibrary.Normal` (- (`self.K2_GetActorLocation` (`GameplayStatics.GetPlayerCharacter` 0)) (`self.K2_GetActorLocation` self))) 5000000.0))))

(fn `Damageint`
  (params (DamageNum :type Integer))
  (returns (`Dead?` :type Boolean))
  (bind _output_get (set `self.Health` (- (`self.Health`) DamageNum)))
  (return (<= _output_get 0)))

(fn `UserConstructionScript`)