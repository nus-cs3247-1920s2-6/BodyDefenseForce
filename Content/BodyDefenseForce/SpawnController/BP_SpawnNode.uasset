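; BP_SpawnNode is a roaming AI spawner that keeps a pack of up to about ten BP_SpawnDrone pawns around it.
; Tick uses delays to spawn drones at nearby navigable points, registering itself as their controller; DroneDown removes dead ones from the set.
; It wanders via a self-restarting AIMoveTo, loosely bounded around its start location, and jumps then chases players it sees.
; Any damage destroys it and sends KillSignal to every drone.
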(event `self.ReceiveTick`
  (params (DeltaSeconds :type "Float (single-precision)"))
  ;[1 1 1] Spawns a Drone when limit is not reached
  (`KismetSystemLibrary.Delay` 0.2)
  (if (< (`BlueprintSetLibrary.Set_Length` (`self.DroneSet`)) 10)
    (`KismetSystemLibrary.Delay` (`KismetMathLibrary.RandomFloatInRange` 0.0 3.0))
    (bind _returnvalue (`AIBlueprintHelperLibrary.SpawnAIFromClass` "/Game/BodyDefenseForce/SpawnController/BP_SpawnDrone.BP_SpawnDrone_C" null (`NavigationSystemV1.K2_GetRandomLocationInNavigableRadius` (`self.K2_GetActorLocation`) 500.0 null null)))
    (bind _asbp_spawn_drone (cast `/Game/BodyDefenseForce/SpawnController/BP_SpawnDrone` _returnvalue)
      (:`then`
        (`/Game/BodyDefenseForce/SpawnController/BPI_Drone.Register Control` _asbp_spawn_drone self)
        (`BlueprintSetLibrary.Set_Add` (`self.DroneSet`) _asbp_spawn_drone))
      (:`CastFailed`
        (`KismetSystemLibrary.PrintString` "ERROR Cast Failed")))))

(event `self.ReceiveAnyDamage`
  (params (Damage :type "Float (single-precision)") (DamageType :type "DamageType Object Reference") (InstigatedBy :type "Controller Object Reference") (DamageCauser :type "Actor Object Reference"))
  ;[1 1 1] When destroyed, kill all drones
  (bind _result (`BlueprintSetLibrary.Set_ToArray` (`self.DroneSet`)))
  (for _array_element _result
    (`/Game/BodyDefenseForce/SpawnController/BPI_Drone.Kill Signal` _array_element))
  (`self.K2_DestroyActor`))

(event `/Game/BodyDefenseForce/SpawnController/BPI_ControlNode.Drone Down`
  (params (`Target Drone` :type "/Game/BodyDefenseForce/SpawnController/BPI_Drone Interface"))
  (bind _droneset (`self.DroneSet`))
  ;[1 1 1] Logs Drone Death
  (bind _asbp_spawn_drone (cast `/Game/BodyDefenseForce/SpawnController/BP_SpawnDrone` `Target Drone`))
  (bind _returnvalue (`BlueprintSetLibrary.Set_Remove` _droneset _asbp_spawn_drone))
  (if _returnvalue
    (`KismetSystemLibrary.PrintString` (`KismetStringLibrary.Conv_IntToString` (`BlueprintSetLibrary.Set_Length` _droneset)))))

(event `self.PawnSensing.OnSeePawn`
  (params (Pawn :type "Pawn Object Reference"))
  ;[1 1 1] On sensing player
  (bind _asdemo_third_person_character (cast `/Game/ThirdPersonCPP/Blueprints/DemoThirdPersonCharacter` Pawn))
  (`self.Jump` self)
  (`|AIMoveTo` self (0.0 0.0 0.0) _asdemo_third_person_character))

(event `self.ReceiveBeginPlay`
  ;[1 1 1] Patrol within fixed radius
  (set `self.InitialLocation` (`self.K2_GetActorLocation`))
  (set `self.BaseJumpVelocity` 0.0)
  (`self.Random Walking`))

(event `Random Walking`
  ;[1 1 1] Patrol within fixed radius
  (bind _location (`self.Random Location`))
  (`|AIMoveTo` self _location null
    (:`OnSuccess`
      _)
    (:`OnFail`
      _))
  (`self.Random Walking`))

(fn `Random Location`
  (returns (location :type "Vector Structure"))
  (bind (_initiallocation_x _initiallocation_y) (`KismetMathLibrary.BreakVector` (`self.InitialLocation`)))
  (bind _randomlocation (`NavigationSystemV1.K2_GetRandomLocationInNavigableRadius` (`self.K2_GetActorLocation`) 1000.0 null null))
  (if (and (<= (`KismetMathLibrary.Abs` (.x _randomlocation)) (+ (`KismetMathLibrary.Abs` _initiallocation_x) 1500.0)) (<= (`KismetMathLibrary.Abs` (.y _randomlocation)) (+ (`KismetMathLibrary.Abs` _initiallocation_y) 1500.0)))
    (return _randomlocation)))

(fn `UserConstructionScript`)