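; BP_PatrolEye is a patrol enemy that detects the player and can be destroyed by damage.
; On BeginPlay it takes its starting and maximum health from its BP_EnemyHealthBar widget.
; Damage, except from BP_AmmoSpawnNode, lowers clamped health and updates the bar; at zero it calls WhenDestroyed on its PatrolEye_AI controller, then destroys itself.
; The SphereOfInfluence overlap sets PlayerSeen when DemoThirdPersonCharacter enters.
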(event `self.ReceiveBeginPlay`
  (`parent.ReceiveBeginPlay`)
  (bind _asbp_enemy_health_bar (cast `/Game/BodyDefenseForce/SpawnController/BP_EnemyHealthBar` (`WidgetComponent.GetUserWidgetObject` (`self.HealthBar`))))
  (set `self.healthBarVar` _asbp_enemy_health_bar)
  (bind _output_get (set `self.health` (`/Game/BodyDefenseForce/SpawnController/BP_EnemyHealthBar.health` _asbp_enemy_health_bar)))
  (set `self.maxHealth` (`/Game/BodyDefenseForce/SpawnController/BP_EnemyHealthBar.maxHealth` _asbp_enemy_health_bar))
  (`/Game/BodyDefenseForce/SpawnController/BP_EnemyHealthBar.UpdateHealth` _asbp_enemy_health_bar _output_get))

(event `self.ReceiveAnyDamage`
  (params (Damage :type "Float (single-precision)") (DamageType :type "DamageType Object Reference") (InstigatedBy :type "Controller Object Reference") (DamageCauser :type "Actor Object Reference"))
  (bind _health (`self.health`))
  ;[1 1 1] Need X shots to kill this thing
  (cast `/Game/ThirdPersonCPP/Blueprints/AmmoSystem/BP_AmmoSpawnNode` DamageCauser
    (:`CastFailed`
      (`self.ModifyHealth` Damage)
      (`/Game/BodyDefenseForce/SpawnController/BP_EnemyHealthBar.UpdateHealth` (`self.healthBarVar`) _health)
      (if (<= (`KismetMathLibrary.FTrunc` _health) 0)
        (bind _aspatrol_eye_ai (cast `/Game/BodyDefenseForce/SpawnController/PatrolAI/PatrolEye_AI` (`AIBlueprintHelperLibrary.GetAIController` self)))
        (`/Game/BodyDefenseForce/SpawnController/PatrolAI/PatrolThing_AI.WhenDestroyed` _aspatrol_eye_ai)
        (`self.K2_DestroyActor`)))))

(event `self.SphereOfInfluence.OnComponentBeginOverlap`
  (params (OverlappedComponent :type "PrimitiveComponent Object Reference") (OtherActor :type "Actor Object Reference") (OtherComp :type "PrimitiveComponent Object Reference") (OtherBodyIndex :type Integer) (bFromSweep :type Boolean) (SweepResult :type "HitResult Structure (by ref)"))
  (cast `/Game/ThirdPersonCPP/Blueprints/DemoThirdPersonCharacter` OtherActor)
  (set `self.PlayerSeen` true))

(fn `ModifyHealth`
  (params (damage :type "Float (double-precision)"))
  (set `self.health` (`KismetMathLibrary.FClamp` (- (`self.health`) damage) 0.0 (`self.maxHealth`))))

(fn `UserConstructionScript`
  (`parent.UserConstructionScript`))