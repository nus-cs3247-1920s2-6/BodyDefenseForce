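; BP_SpawnDrone is an enemy drone that damages the player on contact and belongs to a parent spawn node.
; RegisterControl stores that parent, which is notified through DroneDown when any damage destroys the drone and awards the player XP.
; Box overlap applies damage once until an end overlap resets the attack flag; the trailing random delay triggers nothing.
; KillSignal destroys the drone without notification or XP.
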(event `/Game/BodyDefenseForce/SpawnController/BPI_Drone.Kill Signal`
  (`self.K2_DestroyActor`))

(event `self.ReceiveAnyDamage`
  (params (Damage :type "Float (single-precision)") (DamageType :type "DamageType Object Reference") (InstigatedBy :type "Controller Object Reference") (DamageCauser :type "Actor Object Reference"))
  (`/Game/BodyDefenseForce/SpawnController/BPI_ControlNode.Drone Down` (`self.ParentNode`) self)
  (`self.K2_DestroyActor`)
  (bind _asdemo_third_person_character (cast `/Game/ThirdPersonCPP/Blueprints/DemoThirdPersonCharacter` (`GameplayStatics.GetPlayerCharacter` 0)))
  (`/Game/ThirdPersonCPP/Blueprints/DemoThirdPersonCharacter.AddXP` _asdemo_third_person_character 10.0))

(event `/Game/BodyDefenseForce/SpawnController/BPI_Drone.Register Control`
  (params (`Parent Node` :type "/Game/BodyDefenseForce/SpawnController/BP_SpawnNode Object Reference"))
  (bind _output_get (set `self.ParentNode` `Parent Node`))
  (`KismetSystemLibrary.PrintString` (`KismetSystemLibrary.GetDisplayName` _output_get)))

(event `self.Box.OnComponentBeginOverlap`
  (params (OverlappedComponent :type "PrimitiveComponent Object Reference") (OtherActor :type "Actor Object Reference") (OtherComp :type "PrimitiveComponent Object Reference") (OtherBodyIndex :type Integer) (bFromSweep :type Boolean) (SweepResult :type "HitResult Structure (by ref)"))
  ;[1 1 1] Attacking player
  (bind _asdemo_third_person_character (cast `/Game/ThirdPersonCPP/Blueprints/DemoThirdPersonCharacter` OtherActor))
  (if (not (`self.isAttacking`))
    (set `self.isAttacking` true)
    (`GameplayStatics.ApplyDamage` _asdemo_third_person_character 5.0 null self)
    (`KismetSystemLibrary.Delay` (`KismetMathLibrary.RandomFloatInRange` 0.0 2.0))))

(event `self.Box.OnComponentEndOverlap`
  (params (OverlappedComponent :type "PrimitiveComponent Object Reference") (OtherActor :type "Actor Object Reference") (OtherComp :type "PrimitiveComponent Object Reference") (OtherBodyIndex :type Integer))
  ;[1 1 1] Attacking player
  (set `self.isAttacking` false))

(fn `UserConstructionScript`)