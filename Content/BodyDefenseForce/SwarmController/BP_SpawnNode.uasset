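; BP_SpawnNode is a spawner actor that keeps up to ten BP_SpawnDrone AI pawns alive around itself.
; A delayed Tick spawns drones at random navigable points nearby, registers itself as their controller and tracks them in a set.
; DroneDown removes a reported drone from the set, freeing a slot for replacement.
; Any damage to the node sends KillSignal to every tracked drone, then destroys the node.
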(event `self.ReceiveTick`
  (params (DeltaSeconds :type "Float (single-precision)"))
  ;[1 1 1] Spawns a Drone when limit is not reached
  (`KismetSystemLibrary.Delay` 0.2)
  (if (< (`BlueprintSetLibrary.Set_Length` (`self.DroneSet`)) 10)
    (bind _returnvalue (`AIBlueprintHelperLibrary.SpawnAIFromClass` "/Game/BodyDefenseForce/SwarmController/BP_SpawnDrone.BP_SpawnDrone_C" null (`NavigationSystemV1.K2_GetRandomLocationInNavigableRadius` (`self.K2_GetActorLocation`) 500.0 null null)))
    (bind _asbp_spawn_drone (cast `/Game/BodyDefenseForce/SwarmController/BP_SpawnDrone` _returnvalue)
      (:`then`
        (`/Game/BodyDefenseForce/SwarmController/BPI_Drone.Register Control` _asbp_spawn_drone self)
        (`BlueprintSetLibrary.Set_Add` (`self.DroneSet`) _asbp_spawn_drone))
      (:`CastFailed`
        (`KismetSystemLibrary.PrintString` "ERROR Cast Failed")))))

(event `self.ReceiveAnyDamage`
  (params (Damage :type "Float (single-precision)") (DamageType :type "DamageType Object Reference") (InstigatedBy :type "Controller Object Reference") (DamageCauser :type "Actor Object Reference"))
  ;[1 1 1] When destroyed, kill all drones
  (bind _result (`BlueprintSetLibrary.Set_ToArray` (`self.DroneSet`)))
  (for _array_element _result
    (`/Game/BodyDefenseForce/SwarmController/BPI_Drone.Kill Signal` _array_element))
  (`self.K2_DestroyActor`))

(event `/Game/BodyDefenseForce/SwarmController/BPI_ControlNode.Drone Down`
  (params (`Target Drone` :type "/Game/BodyDefenseForce/SwarmController/BPI_Drone Interface"))
  (bind _droneset (`self.DroneSet`))
  ;[1 1 1] Logs Drone Death
  (bind _asbp_spawn_drone (cast `/Game/BodyDefenseForce/SwarmController/BP_SpawnDrone` `Target Drone`))
  (bind _returnvalue (`BlueprintSetLibrary.Set_Remove` _droneset _asbp_spawn_drone))
  (if _returnvalue
    (`KismetSystemLibrary.PrintString` (`KismetStringLibrary.Conv_IntToString` (`BlueprintSetLibrary.Set_Length` _droneset)))))

(fn `UserConstructionScript`)