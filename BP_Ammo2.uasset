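; BP_Ammo2 is an explosive ammo actor that damages what it hits and blows up.
; On BeginPlay it records its spawn time, sets its attack value and starts a timed self-destruct.
; Box overlaps are ignored for a brief window after spawn; later ones apply damage if the other actor can be damaged, then self-destruct either way.
; SelfDestruct spawns an explosion emitter, plays a 2D sound and destroys the actor.
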(event `self.ReceiveBeginPlay`
  ;[1 0 0.1406] Self Destruct
  (set `self.lifetime` (`KismetSystemLibrary.GetGameTimeInSeconds`))
  (set `self.AttackPoint` 3)
  (`KismetSystemLibrary.Delay` 15.0)
  (`self.SelfDestruct`))

(event `SelfDestruct`
  ;[0.5234 0 1] SelfDestruct
  (`GameplayStatics.SpawnEmitterAtLocation` "/Game/StarterContent/Particles/P_Explosion.P_Explosion" (`self.K2_GetActorLocation`) (struct) (2.0 2.0 2.0))
  (`GameplayStatics.PlaySound2D` "/Game/StarterContent/Audio/Explosion_Cue.Explosion_Cue" 1.0 1.0 0.0 null null)
  (`self.K2_DestroyActor`))

(event `self.Box.OnComponentBeginOverlap`
  (params (OverlappedComponent :type "PrimitiveComponent Object Reference") (OtherActor :type "Actor Object Reference") (OtherComp :type "PrimitiveComponent Object Reference") (OtherBodyIndex :type Integer) (bFromSweep :type Boolean) (SweepResult :type "HitResult Structure (by ref)"))
  ;[0.8516 1 0] Comment
  (if (> (- (`KismetSystemLibrary.GetGameTimeInSeconds`) (`self.lifetime`)) 0.1)
    (if (`Actor.bCanBeDamaged` OtherActor)
      (`GameplayStatics.ApplyDamage` OtherActor (`KismetMathLibrary.Conv_IntToDouble` (`self.AttackPoint`)))
      (`self.SelfDestruct`)
      (else
        (`self.SelfDestruct`)))))

(fn `UserConstructionScript`)