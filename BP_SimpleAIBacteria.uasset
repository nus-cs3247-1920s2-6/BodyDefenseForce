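; Simple enemy AI bacteria that chases the player, deals repeated melee damage, and can optionally spawn copies of itself.
; AISearch drives AIMoveTo with retry on failure, while AttackField overlap stops movement and loops timed damage until overlap ends, then resumes the chase.
; Incoming damage reduces health through the Damageint message, with lethal hits triggering explosion, sound, ragdoll physics and delayed destruction.
; Tick handles timer-based duplication, marked unfinished.
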(event `self.ReceiveBeginPlay`
  ;[0.875 0 1] Set Initialization
  (set `self.BornTime` (`KismetSystemLibrary.GetGameTimeInSeconds`))
  (set `self.Health` (`self.MaxHealth`))
  (`KismetSystemLibrary.Delay` 1.0)
  (set `CharacterMovementComponent.MaxWalkSpeed` (`KismetMathLibrary.RandomFloatInRange` 300.0 500.0) (`self.CharacterMovement`))
  (`self.AISearch`))

(event `AISearch`
  ;[1 0 0.04687] Search
  (if (not (`self.IsDead?`))
    (bind _asdemo_third_person_character (cast `/Game/ThirdPersonCPP/Blueprints/DemoThirdPersonCharacter` (`GameplayStatics.GetPlayerCharacter` 0)))
    (`|AIMoveTo` self (0.0 0.0 0.0) _asdemo_third_person_character :!label _label
      (:`OnFail`
        (`KismetSystemLibrary.Delay` 1.0)
        (goto _label)))))

(event `self.AttackField.OnComponentBeginOverlap`
  (params (OverlappedComponent :type "PrimitiveComponent Object Reference") (OtherActor :type "Actor Object Reference") (OtherComp :type "PrimitiveComponent Object Reference") (OtherBodyIndex :type Integer) (bFromSweep :type Boolean) (SweepResult :type "HitResult Structure (by ref)"))
  ;[0 1 0.2031] AttackBox
  (set `self.IsAttacking?` true)
  (`MovementComponent.StopMovementImmediately` (`self.CharacterMovement`))
  (if (and (`self.IsAttacking?`) (not (`self.IsDead?`))) :!label _label_2
    (`GameplayStatics.ApplyDamage` (`GameplayStatics.GetPlayerCharacter` 0) 5.0 null self)
    (`KismetSystemLibrary.Delay` 1.0)
    (goto _label_2)
    (else
      (`self.AISearch`))))

(event `self.AttackField.OnComponentEndOverlap`
  (params (OverlappedComponent :type "PrimitiveComponent Object Reference") (OtherActor :type "Actor Object Reference") (OtherComp :type "PrimitiveComponent Object Reference") (OtherBodyIndex :type Integer))
  ;[0 1 0.2031] AttackBox
  (set `self.IsAttacking?` false))

(event `self.ReceiveAnyDamage`
  (params (Damage :type "Float (single-precision)") (DamageType :type "DamageType Object Reference") (InstigatedBy :type "Controller Object Reference") (DamageCauser :type "Actor Object Reference"))
  ;[0.1016 1 0] Damage
  (bind _dead_ (message `/Game/BodyDefenseForce/BPI_DamageCalculate.Damageint` self (`KismetMathLibrary.FTrunc` Damage)))
  (if _dead_
    (`MovementComponent.StopMovementImmediately` (`self.CharacterMovement`))
    (`GameplayStatics.SpawnEmitterAtLocation` "/Game/StarterContent/Particles/P_Explosion.P_Explosion" (`self.K2_GetActorLocation`))
    (`GameplayStatics.PlaySoundAtLocation` "/Game/HumanVocalizations/HumanMaleB/Cues/voice_male_b_death_low_03_Cue.voice_male_b_death_low_03_Cue" (0.0 0.0 0.0) (struct) 1.0 1.0 0.0 null null null)
    (`PrimitiveComponent.SetSimulatePhysics` (`self.Mesh`) true)
    (`PrimitiveComponent.SetEnableGravity` (`self.Mesh`) true)
    (`KismetSystemLibrary.Delay` 2.0)
    (`self.K2_DestroyActor`)))

(event `self.ReceiveTick`
  (params (DeltaSeconds :type "Float (single-precision)"))
  ;[1 0 0.75] Duplication(Not Finished)
  (if (`self.CanDuplicate?`)
    (if (`self.Duplicated?`)
      (set `self.Duplicated?` false)
      (set `self.BornTime` (`KismetSystemLibrary.GetGameTimeInSeconds`))
      (else
        (bind _output_get (set `self.TimeCircle` (- (`KismetSystemLibrary.GetGameTimeInSeconds`) (`self.BornTime`))))
        (if (> _output_get (`self.DuplicationTime`))
          (`|SpawnActorFromClass` "BP_SimpleAIBacteria_C" (`KismetMathLibrary.MakeTransform` (+ (`self.K2_GetActorLocation`) (100.0 100.0 0.0))) "AdjustIfPossibleButAlwaysSpawn" "OverrideRootScale" null null)
          (set `self.Duplicated?` true))))))

(fn `Damageint`
  (params (DamageNum :type Integer))
  (returns (`Dead?` :type Boolean))
  (bind _output_get (set `self.Health` (- (`self.Health`) DamageNum)))
  (return (<= _output_get 0)))

(fn `UserConstructionScript`)